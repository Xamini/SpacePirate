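; Randomized roguelike loot drop that rolls rarity and type on BeginPlay: gold, consumable or armor (Weapon falls through to armor).
; Gold scatters denominated Gold_Actors and self-destroys; armor rolls stats, with a malus if both stats match, and tints its mesh and widget by rarity.
; In range, custom depth highlights the item.
; Tick polls Interact, then grants health or keys, or copies armor data to render actors and player materials, and destroys itself.
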(event `self.ReceiveBeginPlay`
  (`self.Hide Meshes`)
  (`SceneComponent.SetVisibility` (`self.Widget`) false false)
  (`self.Choose_Random_Loot`))

(event `Choose_Random_Loot`
  (bind _rarity_output (`self.Choose Rarity` 0))
  (set `self.Rarity` _rarity_output)
  (bind _loot_type (`self.Choose_Item_Type`))
  (bind _output_get (set `self.Item_Type` _loot_type))
  (bind (_item_type_name_txt _primary_stat_txt_value _rarity_txt_value _secondary_stat_txt_value _item_color_value) (`self.Choose_Item` _output_get))
  (set `self.Armor_Type_Name` _item_type_name_txt)
  (set `self.Primary_Stat_TXT` _primary_stat_txt_value)
  (set `self.Rarity_Txt` _rarity_txt_value)
  (set `self.Secondary_Stat_TXT` _secondary_stat_txt_value)
  (set `self.Item_Color_Value` _item_color_value))

(event `self.ReceiveTick`
  (params (DeltaSeconds :type "Float (single-precision)"))
  (bind _asplayer_character (cast `/Game/RogueLike_Game/Character/Player/Blueprints/Player_Character` (`GameplayStatics.GetPlayerCharacter` 0)))
  (if (`self.PlayerCanInteract?`)
    (if (`/Game/RogueLike_Game/Character/Player/Blueprints/Player_Character.Interact?` _asplayer_character)
      (set `self.PlayerCanInteract?` false)
      (if (`|EnumEquality` (`self.Item_Type`) "NewEnumerator1")
        (`self.Consommable_Loot_Interaction`)
        (`self.K2_DestroyActor` :!label _label)
        (elif (`|EnumEquality` (`self.Item_Type`) "NewEnumerator2")
          (`self.Armor_Loot_Interaction`)
          (goto _label))))))

(event `Player_Can_Interact`
  (bind _mesh_picked (`self.Mesh_Picked`))
  (if (`|EnumEquality` (`self.Item_Type`) "NewEnumerator2")
    (`SceneComponent.SetVisibility` (`self.Widget`) true false))
  (set `self.PlayerCanInteract?` true)
  (`PrimitiveComponent.SetRenderCustomDepth` _mesh_picked true)
  (`PrimitiveComponent.SetCustomDepthStencilValue` _mesh_picked 1))

(event `End_Surbrillance`
  (bind _mesh_picked (`self.Mesh_Picked`))
  (`SceneComponent.SetVisibility` (`self.Widget`) false false)
  (`PrimitiveComponent.SetRenderCustomDepth` _mesh_picked false)
  (`PrimitiveComponent.SetCustomDepthStencilValue` _mesh_picked 0)
  (set `self.PlayerCanInteract?` false))

(fn `Armor_Loot_Interaction`
  (if (`|EnumEquality` (`self.Armor_Type`) "NewEnumerator2")
    (bind _returnvalue (`GameplayStatics.GetActorOfClass` "/Game/RogueLike_Game/Character/Player/Widgets/Inventaire/Helmet/Helmet_Render_Actor.Helmet_Render_Actor_C"))
    (`MaterialInstanceDynamic.SetVectorParameterValue` (`/Game/RogueLike_Game/Character/Player/Widgets/Inventaire/Helmet/Helmet_Render_Actor.Inventory_Dynamic_Material` _returnvalue) "Item_Color" (`self.Item_Color_Value`))
    (set `/Game/RogueLike_Game/Character/Player/Widgets/Inventaire/Helmet/Helmet_Render_Actor.Primary_Stat_TXT` (`self.Primary_Stat_TXT`) _returnvalue)
    (set `/Game/RogueLike_Game/Character/Player/Widgets/Inventaire/Helmet/Helmet_Render_Actor.Rarity_Txt` (`self.Rarity_Txt`) _returnvalue)
    (set `/Game/RogueLike_Game/Character/Player/Widgets/Inventaire/Helmet/Helmet_Render_Actor.Item_Type_Name` (`self.Armor_Type_Name`) _returnvalue)
    (set `/Game/RogueLike_Game/Character/Player/Widgets/Inventaire/Helmet/Helmet_Render_Actor.Secondary_Stat_TXT` (`self.Secondary_Stat_TXT`) _returnvalue)
    (set `/Game/RogueLike_Game/Character/Player/Widgets/Inventaire/Helmet/Helmet_Render_Actor.Item_Color` (`self.Item_Color_Value`) _returnvalue)
    (set `/Game/RogueLike_Game/Character/Player/Widgets/Inventaire/Helmet/Helmet_Render_Actor.Primary_Stat_Type` (`self.Primary_Stat_Type`) _returnvalue)
    (set `/Game/RogueLike_Game/Character/Player/Widgets/Inventaire/Helmet/Helmet_Render_Actor.Secondary_Stat_Type` (`self.Secondary_Stat_Type`) _returnvalue)
    (set `/Game/RogueLike_Game/Character/Player/Widgets/Inventaire/Helmet/Helmet_Render_Actor.Primary_Stat_Value` (`self.Primary_Stat_Value`) _returnvalue)
    (set `/Game/RogueLike_Game/Character/Player/Widgets/Inventaire/Helmet/Helmet_Render_Actor.Secondary_Stat_Value` (`self.Secondary_Stat_Value`) _returnvalue)
    (set `/Game/RogueLike_Game/Character/Player/Widgets/Inventaire/Helmet/Helmet_Render_Actor.Secondary_Stat_Negative?` (`self.Secondary_Stat_Negative?`) _returnvalue)
    (bind _asplayer_character (cast `/Game/RogueLike_Game/Character/Player/Blueprints/Player_Character` (`GameplayStatics.GetPlayerCharacter` 0)))
    (`MaterialInstanceDynamic.SetVectorParameterValue` (`/Game/RogueLike_Game/Character/Player/Blueprints/Player_Character.Helmet_Rarity_Material` _asplayer_character) "Item_Color" (`self.Item_Color_Value`))
    (else
      (bind _returnvalue_2 (`GameplayStatics.GetActorOfClass` "/Game/RogueLike_Game/Character/Player/Widgets/Inventaire/ChestPlate/ChestPlate_Render_Actor.ChestPlate_Render_Actor_C"))
      (`MaterialInstanceDynamic.SetVectorParameterValue` (`/Game/RogueLike_Game/Character/Player/Widgets/Inventaire/ChestPlate/ChestPlate_Render_Actor.Inventory_Dynamic_Material` _returnvalue_2) "Item_Color" (`self.Item_Color_Value`))
      (set `/Game/RogueLike_Game/Character/Player/Widgets/Inventaire/ChestPlate/ChestPlate_Render_Actor.Primary_Stat_TXT` (`self.Primary_Stat_TXT`) _returnvalue_2)
      (set `/Game/RogueLike_Game/Character/Player/Widgets/Inventaire/ChestPlate/ChestPlate_Render_Actor.Rarity_Txt` (`self.Rarity_Txt`) _returnvalue_2)
      (set `/Game/RogueLike_Game/Character/Player/Widgets/Inventaire/ChestPlate/ChestPlate_Render_Actor.Item_Type_Name` (`self.Armor_Type_Name`) _returnvalue_2)
      (set `/Game/RogueLike_Game/Character/Player/Widgets/Inventaire/ChestPlate/ChestPlate_Render_Actor.Secondary_Stat_TXT` (`self.Secondary_Stat_TXT`) _returnvalue_2)
      (set `/Game/RogueLike_Game/Character/Player/Widgets/Inventaire/ChestPlate/ChestPlate_Render_Actor.Item_Color` (`self.Item_Color_Value`) _returnvalue_2)
      (set `/Game/RogueLike_Game/Character/Player/Widgets/Inventaire/ChestPlate/ChestPlate_Render_Actor.Primary_Stat_Type` (`self.Primary_Stat_Type`) _returnvalue_2)
      (set `/Game/RogueLike_Game/Character/Player/Widgets/Inventaire/ChestPlate/ChestPlate_Render_Actor.Secondary_Stat_Type` (`self.Secondary_Stat_Type`) _returnvalue_2)
      (set `/Game/RogueLike_Game/Character/Player/Widgets/Inventaire/ChestPlate/ChestPlate_Render_Actor.Primary_Stat_Value` (`self.Primary_Stat_Value`) _returnvalue_2)
      (set `/Game/RogueLike_Game/Character/Player/Widgets/Inventaire/ChestPlate/ChestPlate_Render_Actor.Secondary_Stat_Value` (`self.Secondary_Stat_Value`) _returnvalue_2)
      (set `/Game/RogueLike_Game/Character/Player/Widgets/Inventaire/ChestPlate/ChestPlate_Render_Actor.Secondary_Stat_Negative?` (`self.Secondary_Stat_Negative?`) _returnvalue_2)
      (bind _asplayer_character_2 (cast `/Game/RogueLike_Game/Character/Player/Blueprints/Player_Character` (`GameplayStatics.GetPlayerCharacter` 0)))
      (`MaterialInstanceDynamic.SetVectorParameterValue` (`/Game/RogueLike_Game/Character/Player/Blueprints/Player_Character.ChestPlate_Rarity_Material` _asplayer_character_2) "Item_Color" (`self.Item_Color_Value`)))))

(fn `Choose Rarity`
  (params (Rarity_Chance :type Integer))
  (returns (Rarity_Output :type "/Game/RogueLike_Game/Blueprints/Loot/Enum/Rarity_Enum Enum"))
  (locals (Random_Int :type Integer))
  (bind _output_get (set `local.Random_Int` (`KismetMathLibrary.RandomIntegerInRange` 1 100)))
  (if (<= _output_get (- 40 Rarity_Chance))
    (return "NewEnumerator0")
    (elif (<= (`local.Random_Int`) (- 70 Rarity_Chance))
      (return "NewEnumerator1")
      (elif (<= (`local.Random_Int`) (- 90 Rarity_Chance))
        (return "NewEnumerator2")
        (else
          (return "NewEnumerator3"))))))

(fn `Choose_Armor_Statistics`
  (params (Armor_Type :type "/Game/RogueLike_Game/Blueprints/Loot/Enum/Armor_Type_Enum Enum" :default "NewEnumerator2") (Rarity :type "/Game/RogueLike_Game/Blueprints/Loot/Enum/Rarity_Enum Enum" :default "NewEnumerator0"))
  (returns (Primary_Stat_Type :type "/Game/RogueLike_Game/Blueprints/Loot/Enum/Statistics_Type Enum") (Primary_Stat_Value :type Integer) (Secondary_Stat_Type :type "/Game/RogueLike_Game/Blueprints/Loot/Enum/Statistics_Type Enum") (Secondary_Stat_Value :type Integer))
  (locals (Primary_Stat_Value_Setting :type Integer :default 0) (Secondary_Stat_Type_Setting :type "/Game/RogueLike_Game/Blueprints/Loot/Enum/Statistics_Type Enum" :default "NewEnumerator0") (Primary_Stat_Bonus :type "Map of /Game/RogueLike_Game/Blueprints/Loot/Enum/Rarity_Enum Enum to Integer"))
  (bind _secondary_stat_type_map (`self.Secondary_Stat_Type_Map`))
  (bind _value (`BlueprintMapLibrary.Map_Find` (`self.Secondary_Stat_Value_Map`) Rarity))
  (bind _value_2 (`BlueprintMapLibrary.Map_Find` (`self.Primary_Stat_Type_Map`) Armor_Type))
  (bind _value_3 (`BlueprintMapLibrary.Map_Find` (`self.Primary_Stat_Value_Map`) Rarity))
  (bind _output_get (set `local.Secondary_Stat_Type_Setting` (`|GetArrayItem` _secondary_stat_type_map (`KismetMathLibrary.RandomIntegerInRange` 0 (`KismetArrayLibrary.Array_LastIndex` _secondary_stat_type_map)))))
  (if (`|EnumEquality` _value_2 _output_get)
    (set `local.Primary_Stat_Value_Setting` (`BlueprintMapLibrary.Map_Find` (`local.Primary_Stat_Bonus`) Rarity))
    (set `local.Secondary_Stat_Type_Setting` (`BlueprintMapLibrary.Map_Find` (`self.Malus_Stat_Type`) _value_2))
    (set `self.Secondarity_Stat_PosNeg` "  -")
    (set `self.Secondary_Stat_Negative?` true)
    (else
      (set `local.Primary_Stat_Value_Setting` (`KismetMathLibrary.RandomIntegerInRange` (`KismetMathLibrary.FTrunc` (.x _value_3)) (`KismetMathLibrary.FTrunc` (.y _value_3))))
      (set `self.Secondarity_Stat_PosNeg` "  +")))
  (return _value_2 (`local.Primary_Stat_Value_Setting`) (`local.Secondary_Stat_Type_Setting`) (`KismetMathLibrary.RandomIntegerInRange` (`KismetMathLibrary.FTrunc` (.x _value)) (`KismetMathLibrary.FTrunc` (.y _value)))))

(fn `Choose_Armor_Type`
  (returns (Armor_Type :type "/Game/RogueLike_Game/Blueprints/Loot/Enum/Armor_Type_Enum Enum"))
  (return (select `int` (`KismetMathLibrary.RandomIntegerInRange` 0 1) :`0` "NewEnumerator2" :`1` "NewEnumerator3" :`2` "NewEnumerator4" :!type "/Game/RogueLike_Game/Blueprints/Loot/Enum/Armor_Type_Enum Enum")))

(fn `Choose_Consommable_Type`
  (returns (Consommable_Type :type "/Game/RogueLike_Game/Blueprints/Loot/Enum/Consommable_Type Enum"))
  (return (select `int` (`KismetMathLibrary.RandomIntegerInRange` 0 2) :`0` "NewEnumerator0" :`1` "NewEnumerator2" :!type "/Game/RogueLike_Game/Blueprints/Loot/Enum/Consommable_Type Enum")))

(fn `Choose_Item`
  (params (Loot_Type :type "/Game/RogueLike_Game/Blueprints/Chest_Loot/LootType_Enum Enum" :default "NewEnumerator0"))
  (returns (Item_Type_Name_TXT :type Text) (Primary_Stat_TXT_Value :type Text) (Rarity_TXT_Value :type Text) (Secondary_Stat_TXT_Value :type Text) (Item_Color_Value :type "LinearColor Structure"))
  (locals (Item_Color :type "Map of /Game/RogueLike_Game/Blueprints/Loot/Enum/Rarity_Enum Enum to Color Structure") (Min_Drop_Gold :type Integer :default 1) (Max_Drop_Gold :type Integer :default 15) (Stage_Level :type Integer :default 0) (Amount_To_Drop :type Integer :default 23) (Gold_Color_Item :type "Array of LinearColor Structure"))
  (bind _returnvalue (`self.K2_GetActorLocation`))
  (bind _returnvalue_2 (`self.K2_GetActorLocation`))
  (bind _returnvalue_3 (`self.K2_GetActorLocation`))
  (bind _rarity (`self.Rarity`))
  (bind _value (`BlueprintMapLibrary.Map_Find` (`local.Item_Color`) _rarity))
  (bind (_returnvalue_x _returnvalue_y) (`KismetMathLibrary.BreakVector` (`KismetMathLibrary.RandomPointInBoundingBox` _returnvalue (50.0 50.0 30.0))))
  (bind (_returnvalue_x_2 _returnvalue_y_2) (`KismetMathLibrary.BreakVector` (`KismetMathLibrary.RandomPointInBoundingBox` _returnvalue_2 (50.0 50.0 30.0))))
  (bind (_returnvalue_x_3 _returnvalue_y_3) (`KismetMathLibrary.BreakVector` (`KismetMathLibrary.RandomPointInBoundingBox` _returnvalue_3 (50.0 50.0 30.0))))
  (bind _returnvalue_4 (* (`local.Stage_Level`) 5))
  (bind _returnvalue_5 (`KismetTextLibrary.Conv_StringToText` (`|GetEnumeratorNameAsString` (`self.Rarity`))))
  (bind _returnvalue_6 (`KismetMathLibrary.Conv_ColorToLinearColor` _value))
  (switch `/Game/RogueLike_Game/Blueprints/Chest_Loot/LootType_Enum` Loot_Type
    (:`NewEnumerator0`
      ;[1 1 1] Gold_Loot_System
      (set `local.Min_Drop_Gold` (+ _returnvalue_4 (`local.Min_Drop_Gold`)))
      (set `local.Max_Drop_Gold` (+ _returnvalue_4 (`local.Max_Drop_Gold`)))
      (bind _output_get (set `local.Amount_To_Drop` (`KismetMathLibrary.RandomIntegerInRange` (`local.Min_Drop_Gold`) (`local.Max_Drop_Gold`))))
      (bind _returnvalue_7 (- (/ _output_get 10) 1))
      (if (>= _returnvalue_7 0)
        (for _ (range (+ _returnvalue_7 1))
          (`|SpawnActorFromClass` "/Game/RogueLike_Game/Blueprints/Loot/Gold/Gold_Actor.Gold_Actor_C" (`KismetMathLibrary.MakeTransform` (`KismetMathLibrary.MakeVector` _returnvalue_x_2 _returnvalue_y_2 (+ (.z _returnvalue_2) 10.0))) "Undefined" "OverrideRootScale" null (`|GetArrayItem` (`local.Gold_Color_Item`) 2) 10 null)))
      (bind _returnvalue_8 (mod _output_get 10))
      (bind _returnvalue_9 (- (/ _returnvalue_8 5) 1))
      (if (>= _returnvalue_9 0)
        (for _ (range (+ _returnvalue_9 1))
          (`|SpawnActorFromClass` "/Game/RogueLike_Game/Blueprints/Loot/Gold/Gold_Actor.Gold_Actor_C" (`KismetMathLibrary.MakeTransform` (`KismetMathLibrary.MakeVector` _returnvalue_x_3 _returnvalue_y_3 (+ (.z _returnvalue_3) 10.0))) "Undefined" "OverrideRootScale" null (`|GetArrayItem` (`local.Gold_Color_Item`) 1) 5 null)))
      (bind _returnvalue_10 (- (mod _returnvalue_8 5) 1))
      (if (>= _returnvalue_10 0)
        (for _ (range (+ _returnvalue_10 1))
          (`|SpawnActorFromClass` "/Game/RogueLike_Game/Blueprints/Loot/Gold/Gold_Actor.Gold_Actor_C" (`KismetMathLibrary.MakeTransform` (`KismetMathLibrary.MakeVector` _returnvalue_x _returnvalue_y (+ (.z _returnvalue) 10.0))) "Undefined" "OverrideRootScale" null (`|GetArrayItem` (`local.Gold_Color_Item`)) 1 null)))
      (`self.K2_DestroyActor`))
    (:`NewEnumerator1`
      (bind _consommable_type (`self.Choose_Consommable_Type`))
      (bind _output_get_2 (set `self.Consommable_Type` _consommable_type))
      (bind _output_get_3 (set `self.Mesh_Picked` (`BlueprintMapLibrary.Map_Find` (`self.Consommable_Meshes`) _output_get_2)))
      (`SceneComponent.SetVisibility` _output_get_3 true false))
    (:`NewEnumerator2`
      ;[1 1 1] Armor_Loot_System
      (bind _armor_type (`self.Choose_Armor_Type` :!label _label))
      (bind _output_get_4 (set `self.Armor_Type` _armor_type))
      (bind (_primary_stat_type _primary_stat_value _secondary_stat_type _secondary_stat_value) (`self.Choose_Armor_Statistics` _output_get_4 _rarity))
      (set `self.Primary_Stat_Type` _primary_stat_type)
      (set `self.Primary_Stat_Value` _primary_stat_value)
      (set `self.Secondary_Stat_Type` _secondary_stat_type)
      (set `self.Secondary_Stat_Value` _secondary_stat_value)
      (bind _output_get_5 (set `self.Mesh_Picked` (`BlueprintMapLibrary.Map_Find` (`self.Armor_Meshes`) _armor_type)))
      (`SceneComponent.SetVisibility` _output_get_5 true false)
      (bind _asloot_item_widget (cast `/Game/RogueLike_Game/Blueprints/Loot/Loot_Item_Widget` (`WidgetComponent.GetUserWidgetObject` (`self.Widget`))))
      (`Image.SetColorAndOpacity` (`/Game/RogueLike_Game/Blueprints/Loot/Loot_Item_Widget.Background_Color` _asloot_item_widget) (`KismetMathLibrary.Conv_ColorToLinearColor` _value))
      (bind _returnvalue_11 (`KismetTextLibrary.Conv_StringToText` (`|GetEnumeratorNameAsString` _output_get_4)))
      (`TextBlock.SetText` (`/Game/RogueLike_Game/Blueprints/Loot/Loot_Item_Widget.Item_Type_Name` _asloot_item_widget) _returnvalue_11)
      (bind _returnvalue_12 (`KismetTextLibrary.Conv_StringToText` (`KismetStringLibrary.Concat_StrStr` (`|GetEnumeratorNameAsString` _primary_stat_type) "  +" (`KismetStringLibrary.Conv_IntToString` _primary_stat_value))))
      (`TextBlock.SetText` (`/Game/RogueLike_Game/Blueprints/Loot/Loot_Item_Widget.Primary_Stat` _asloot_item_widget) _returnvalue_12)
      (`TextBlock.SetText` (`/Game/RogueLike_Game/Blueprints/Loot/Loot_Item_Widget.Rarity` _asloot_item_widget) _returnvalue_5)
      (bind _returnvalue_13 (`KismetTextLibrary.Conv_StringToText` (`KismetStringLibrary.Concat_StrStr` (`|GetEnumeratorNameAsString` _secondary_stat_type) (`self.Secondarity_Stat_PosNeg`) (`KismetStringLibrary.Conv_IntToString` _secondary_stat_value))))
      (`TextBlock.SetText` (`/Game/RogueLike_Game/Blueprints/Loot/Loot_Item_Widget.Secondary_Stat` _asloot_item_widget) _returnvalue_13)
      (bind _values (`BlueprintMapLibrary.Map_Values` (`self.Armor_Meshes`)))
      (`MaterialInstanceDynamic.SetVectorParameterValue` (`|GetArrayItem` (`self.Armor_Material_Instance`) (`KismetArrayLibrary.Array_Find` _values (`self.Mesh_Picked`))) "Item_Color" _returnvalue_6)
      (return _returnvalue_11 _returnvalue_12 _returnvalue_5 _returnvalue_13 _returnvalue_6))
    (:`NewEnumerator3`
      (goto _label))))

(fn `Choose_Item_Type`
  (returns (Loot_Type :type "/Game/RogueLike_Game/Blueprints/Chest_Loot/LootType_Enum Enum"))
  (locals (Item_Type_List :type "/Game/RogueLike_Game/Blueprints/Loot/Enum/Item_Type_Enum Enum" :default "NewEnumerator0"))
  (return (select `int` (`KismetMathLibrary.RandomIntegerInRange` 0 3) :`0` "NewEnumerator0" :`1` "NewEnumerator1" :`2` "NewEnumerator2" :`3` "NewEnumerator3" :!type "/Game/RogueLike_Game/Blueprints/Chest_Loot/LootType_Enum Enum")))

(fn `Consommable_Loot_Interaction`
  (bind _asplayer_character (cast `/Game/RogueLike_Game/Character/Player/Blueprints/Player_Character` (`GameplayStatics.GetPlayerCharacter` 0)))
  (if (`|EnumEquality` (`self.Consommable_Type`) "NewEnumerator0")
    (set `/Game/RogueLike_Game/Character/Player/Blueprints/Player_Character.HealthPoint` (+ (`/Game/RogueLike_Game/Character/Player/Blueprints/Player_Character.HealthPoint` _asplayer_character) 10) _asplayer_character)
    (else
      (set `/Game/RogueLike_Game/Character/Player/Blueprints/Player_Character.Chest_Keys` (+ (`/Game/RogueLike_Game/Character/Player/Blueprints/Player_Character.Chest_Keys` _asplayer_character) 1) _asplayer_character))))

(fn `Hide Meshes`
  (`|ExecutionSequence`
    (:`then_0`
      (`BlueprintMapLibrary.Map_Add` (`self.Armor_Meshes`) "NewEnumerator2" (`self.Helmet`))
      (`BlueprintMapLibrary.Map_Add` (`self.Armor_Meshes`) "NewEnumerator3" (`self.ChestPlate`)))
    (:`then_1`
      (bind _values (`BlueprintMapLibrary.Map_Values` (`self.Armor_Meshes`)))
      (for _array_element _values
        (`SceneComponent.SetVisibility` _array_element false false)
        (bind _returnvalue (`PrimitiveComponent.CreateDynamicMaterialInstance` _array_element 0 "/Game/RogueLike_Game/Blueprints/Loot/Rarity_Item_Material_Inst.Rarity_Item_Material_Inst" "None"))
        (`KismetArrayLibrary.Array_Add` (`self.Armor_Material_Instance`) _returnvalue)))
    (:`then_2`
      (`BlueprintMapLibrary.Map_Add` (`self.Consommable_Meshes`) "NewEnumerator0" (`self.Health_Potion`))
      (`BlueprintMapLibrary.Map_Add` (`self.Consommable_Meshes`) "NewEnumerator2" (`self.Chest_Key`)))))

(fn `UserConstructionScript`)