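; Gold pickup actor that flies toward the player and adds its Amount to the player character's gold on contact.
; On BeginPlay it creates a dynamic material instance to tint the mesh with its Color.
; Overlapping a component tagged Gold_Attraction_Box starts a timeline that lerps it from its current location toward the player.
; Overlapping a Player_Capsule-tagged component credits the gold and destroys the actor.
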(event `self.ReceiveBeginPlay`
  (bind _returnvalue (`PrimitiveComponent.CreateDynamicMaterialInstance` (`self.Gold`) 0 "/Game/RogueLike_Game/Blueprints/Loot/Gold_Material_Inst.Gold_Material_Inst" "None"))
  (`MaterialInstanceDynamic.SetVectorParameterValue` _returnvalue "Money_Color" (`self.Color`)))

(event `self.Gold.OnComponentBeginOverlap`
  (params (OverlappedComponent :type "PrimitiveComponent Object Reference") (OtherActor :type "Actor Object Reference") (OtherComp :type "PrimitiveComponent Object Reference") (OtherBodyIndex :type Integer) (bFromSweep :type Boolean) (SweepResult :type "HitResult Structure (by ref)"))
  (if (`ActorComponent.ComponentHasTag` OtherComp "Gold_Attraction_Box")
    (bind (_direction _lerp) (`Timeline|Gold_Attraction_Timeline` :!via `PlayFromStart`)
      (:`Update`
        (`SceneComponent.K2_SetWorldLocation` (`self.DefaultSceneRoot`) (`KismetMathLibrary.VLerp` (`self.K2_GetActorLocation`) (`self.K2_GetActorLocation` (`GameplayStatics.GetPlayerCharacter` 0)) _lerp) false false)))
    (elif (`ActorComponent.ComponentHasTag` OtherComp "Player_Capsule")
      (bind _asplayer_character (cast `/Game/RogueLike_Game/Character/Player/Blueprints/Player_Character` (`GameplayStatics.GetPlayerCharacter` 0)))
      (set `/Game/RogueLike_Game/Character/Player/Blueprints/Player_Character.Gold` (+ (`/Game/RogueLike_Game/Character/Player/Blueprints/Player_Character.Gold` _asplayer_character) (`self.Amount`)) _asplayer_character)
      (`self.K2_DestroyActor`))))

(fn `UserConstructionScript`)