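; Roguelike map generator that lays out a random path of instanced rooms on a grid from an entry to an exit when play begins.
; BeginPlay registers each room's corridor openings and fills per-direction candidate pools, then Generate Map builds the free grid cells.
; A delayed loop steps into a free neighbor through the last room's openings and places a random room with a matching opening.
; Each placed room leaves every pool, so none repeats.
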(event `self.ReceiveBeginPlay`
  (`self.Add_Room_Corridor_Infos` (`self.Room_Normal_01`) (make `/Game/RogueLike_Game/Blueprints/Map_Generation/Room_Structure` false true true))
  (`self.Add_Room_Corridor_Infos` (`self.Room_Normal_02`) (make `/Game/RogueLike_Game/Blueprints/Map_Generation/Room_Structure` false true false true))
  (`self.Add_Room_Corridor_Infos` (`self.Room_Normal_03`) (make `/Game/RogueLike_Game/Blueprints/Map_Generation/Room_Structure` false false true true))
  (`self.Add_Room_Corridor_Infos` (`self.Room_Normal_04`) (make `/Game/RogueLike_Game/Blueprints/Map_Generation/Room_Structure` false true false true))
  (`self.Add_Room_Corridor_Infos` (`self.Room_Normal_05`) (make `/Game/RogueLike_Game/Blueprints/Map_Generation/Room_Structure` true true))
  (`self.Add_Room_Corridor_Infos` (`self.Room_Normal_06`) (make `/Game/RogueLike_Game/Blueprints/Map_Generation/Room_Structure` true true))
  (`self.Add_Room_Corridor_Infos` (`self.Room_Normal_07`) (make `/Game/RogueLike_Game/Blueprints/Map_Generation/Room_Structure` false true true))
  (`self.Add_Room_Corridor_Infos` (`self.Room_Normal_08`) (make `/Game/RogueLike_Game/Blueprints/Map_Generation/Room_Structure` true true))
  (`self.Add_Room_Corridor_Infos` (`self.Room_Hub_09`) (make `/Game/RogueLike_Game/Blueprints/Map_Generation/Room_Structure` true true true))
  (`self.Add_Room_Corridor_Infos` (`self.Room_Normal_10`) (make `/Game/RogueLike_Game/Blueprints/Map_Generation/Room_Structure` true false false true))
  (`self.Add_Room_Corridor_Infos` (`self.Room_Hub_11`) (make `/Game/RogueLike_Game/Blueprints/Map_Generation/Room_Structure` false true true true))
  (`self.Add_Room_Corridor_Infos` (`self.Room_End_12`) (make `/Game/RogueLike_Game/Blueprints/Map_Generation/Room_Structure` false true))
  (`self.Add_Room_Corridor_Infos` (`self.Room_Normal_13`) (make `/Game/RogueLike_Game/Blueprints/Map_Generation/Room_Structure` false true true))
  (`self.Add_Room_Corridor_Infos` (`self.Room_Hub_14`) (make `/Game/RogueLike_Game/Blueprints/Map_Generation/Room_Structure` false true true true))
  (`self.Add_Room_Corridor_Infos` (`self.Room_Hub_15`) (make `/Game/RogueLike_Game/Blueprints/Map_Generation/Room_Structure` true true true true))
  (set `self.Normal_Rooms_North` (`|MakeArray` (`self.Room_Normal_05`) (`self.Room_Normal_06`) (`self.Room_Normal_08`) (`self.Room_Hub_09`) (`self.Room_Normal_10`)))
  (set `self.Normal_Rooms_South` (`|MakeArray` (`self.Room_Normal_01`) (`self.Room_Normal_02`) (`self.Room_Normal_04`) (`self.Room_Normal_05`) (`self.Room_Normal_06`) (`self.Room_Normal_07`) (`self.Room_Normal_08`) (`self.Room_Hub_09`) (`self.Room_Hub_11`)))
  (set `self.Normal_Rooms_East` (`|MakeArray` (`self.Room_Normal_01`) (`self.Room_Normal_03`) (`self.Room_Hub_09`) (`self.Room_Hub_11`) (`self.Room_Normal_07`)))
  (set `self.Normal_Rooms_West` (`|MakeArray` (`self.Room_Normal_02`) (`self.Room_Normal_03`) (`self.Room_Normal_04`) (`self.Room_Normal_10`) (`self.Room_Hub_11`)))
  (set `self.Hub_Rooms_North` (`|MakeArray` null null null null :!type "InstancedStaticMeshComponent Object Reference"))
  (`self.Generate_Map`))

(event `Generate_Map`
  (bind _lastcreatedtilelocation (`self.LastCreatedTileLocation`))
  (bind _tile_size (`self.Tile_Size`))
  (bind _tile_size_2 (`self.Tile_Size`))
  (bind _normal_rooms_north (`self.Normal_Rooms_North`))
  (bind _normal_room_picked (`self.Normal_Room_Picked`))
  (bind _lastcreatedtilelocation_2 (`self.LastCreatedTileLocation`))
  (bind _normal_rooms_south (`self.Normal_Rooms_South`))
  (bind _lastcreatedtilelocation_3 (`self.LastCreatedTileLocation`))
  (bind _normal_rooms_east (`self.Normal_Rooms_East`))
  (bind _normal_rooms_west (`self.Normal_Rooms_West`))
  (bind _normal_rooms_west_2 (`self.Normal_Rooms_West`))
  (bind _lastcreatedtilelocation_4 (`self.LastCreatedTileLocation`))
  (bind _tile_size_3 (`self.Tile_Size`))
  (bind _tile_size_4 (`self.Tile_Size`))
  (bind _tile_size_5 (`self.Tile_Size`))
  (bind _tile_size_6 (`self.Tile_Size`))
  (bind _tile_size_7 (`self.Tile_Size`))
  (bind _returnvalue (+ (`self.LastCreatedTileLocation`) (`KismetMathLibrary.MakeVector` 0.0 (+ (* (`self.Room_Size`) _tile_size_3) (* (`self.Distance_Between_Rooms`) _tile_size_3)))))
  (bind _returnvalue_2 (+ (`self.LastCreatedTileLocation`) (`KismetMathLibrary.MakeVector` (+ (* (`self.Room_Size`) _tile_size_6) (* (`self.Distance_Between_Rooms`) _tile_size_6)))))
  (bind _returnvalue_3 (+ (`self.LastCreatedTileLocation`) (`KismetMathLibrary.MakeVector` 0.0 (* (+ (* (`self.Room_Size`) _tile_size_5) (* (`self.Distance_Between_Rooms`) _tile_size_5)) -1.0))))
  (bind _returnvalue_4 (+ (`self.LastCreatedTileLocation`) (`KismetMathLibrary.MakeVector` (* (+ (* (`self.Room_Size`) _tile_size_7) (* (`self.Distance_Between_Rooms`) _tile_size_7)) -1.0))))
  ;[1 1 1] Generate Room Available Location
  (for _index (range (`self.Grid_SizeX`))
    (for _index_2 (range (`self.Grid_SizeY`))
      (`KismetArrayLibrary.Array_Add` (`self.Available_Grid_Location`) (+ (* (`KismetMathLibrary.MakeVector` (+ (* (`self.Room_Size`) _tile_size_2) (* (`self.Distance_Between_Rooms`) _tile_size_2))) _index) (* (`KismetMathLibrary.MakeVector` 0.0 (+ (* (`self.Room_Size`) _tile_size_2) (* (`self.Distance_Between_Rooms`) _tile_size_2))) _index_2)))))
  (bind _output_get (set `self.LastCreatedTileLocation` (`KismetMathLibrary.MakeVector` (* (`KismetMathLibrary.RandomIntegerInRange` 0 (- (`self.Grid_SizeX`) 1)) (+ (* (`self.Room_Size`) _tile_size) (* (`self.Distance_Between_Rooms`) _tile_size))))))
  (`KismetArrayLibrary.Array_RemoveItem` (`self.Available_Grid_Location`) _output_get)
  (`InstancedStaticMeshComponent.AddInstance` (`self.Entry`) (`KismetMathLibrary.MakeTransform` _output_get (struct :`Yaw` -90.0)))
  (bind _index_3 (`self.For Loop With Delay` 0 (`self.Room_Count`))
    (:`LoopBody`
      (if (== _index_3 0)
        (bind _output_get_2 (set `self.LastCreatedTileLocation` (+ (`self.LastCreatedTileLocation`) (`KismetMathLibrary.MakeVector` 0.0 (+ (* (`self.Room_Size`) _tile_size_4) (* (`self.Distance_Between_Rooms`) _tile_size_4))))))
        (bind _output_get_3 (set `self.Normal_Room_Picked` (`|GetArrayItem` _normal_rooms_west_2 (`KismetMathLibrary.RandomIntegerInRange` 0 (- (`KismetArrayLibrary.Array_Length` _normal_rooms_west_2) 1)))))
        (`InstancedStaticMeshComponent.AddInstance` _output_get_3 (`KismetMathLibrary.MakeTransform` _output_get_2))
        (`KismetArrayLibrary.Array_Add` (`self.Created_Room_Location`) _output_get_2)
        (`KismetArrayLibrary.Array_RemoveItem` (`self.Available_Grid_Location`) _output_get_2)
        (`KismetArrayLibrary.Array_RemoveItem` (`self.Normal_Rooms_North`) _output_get_3)
        (`KismetArrayLibrary.Array_RemoveItem` (`self.Normal_Rooms_South`) _output_get_3)
        (`KismetArrayLibrary.Array_RemoveItem` (`self.Normal_Rooms_East`) _output_get_3)
        (`KismetArrayLibrary.Array_RemoveItem` (`self.Normal_Rooms_West`) _output_get_3)
        (else
          (`BlueprintMapLibrary.Map_Clear` (`self.Next_Room_Location`))
          (if (break `/Game/RogueLike_Game/Blueprints/Map_Generation/Room_Structure` (`BlueprintMapLibrary.Map_Find` (`self.Room_Corridor_Entry_Infos`) (`self.Normal_Room_Picked`)))
            (if (`KismetArrayLibrary.Array_Contains` (`self.Available_Grid_Location`) _returnvalue_2)
              (`BlueprintMapLibrary.Map_Add` (`self.Next_Room_Location`) "North" _returnvalue_2)))
          (if (`.South_3_DCC0241B446A85D924B11096E28BCDA3` (break `/Game/RogueLike_Game/Blueprints/Map_Generation/Room_Structure` (`BlueprintMapLibrary.Map_Find` (`self.Room_Corridor_Entry_Infos`) (`self.Normal_Room_Picked`))))
            (if (`KismetArrayLibrary.Array_Contains` (`self.Available_Grid_Location`) _returnvalue_4)
              (`BlueprintMapLibrary.Map_Add` (`self.Next_Room_Location`) "South" _returnvalue_4)))
          (if (`.East_6_0F1263E84CFC3EB3BECD78A5634E4723` (break `/Game/RogueLike_Game/Blueprints/Map_Generation/Room_Structure` (`BlueprintMapLibrary.Map_Find` (`self.Room_Corridor_Entry_Infos`) (`self.Normal_Room_Picked`))))
            (if (`KismetArrayLibrary.Array_Contains` (`self.Available_Grid_Location`) _returnvalue)
              (`BlueprintMapLibrary.Map_Add` (`self.Next_Room_Location`) "East" _returnvalue)))
          (if (`.West_7_556C14CE40AFF1CA6AF804ADD6AF37B6` (break `/Game/RogueLike_Game/Blueprints/Map_Generation/Room_Structure` (`BlueprintMapLibrary.Map_Find` (`self.Room_Corridor_Entry_Infos`) (`self.Normal_Room_Picked`))))
            (if (`KismetArrayLibrary.Array_Contains` (`self.Available_Grid_Location`) _returnvalue_3)
              (`BlueprintMapLibrary.Map_Add` (`self.Next_Room_Location`) "West" _returnvalue_3)))
          (bind _keys (`BlueprintMapLibrary.Map_Keys` (`self.Next_Room_Location`)))
          (bind _output_get_4 (set `self.Next_Room_Picked` (`|GetArrayItem` _keys (`KismetMathLibrary.RandomIntegerInRange` 0 (- (`KismetArrayLibrary.Array_Length` _keys) 1)))))
          (bind _output_get_5 (set `self.LastCreatedTileLocation` (`BlueprintMapLibrary.Map_Find` (`self.Next_Room_Location`) _output_get_4)))
          (if (== _index_3 (`self.Room_Count`))
            (`InstancedStaticMeshComponent.AddInstance` (`self.Exit`) (`KismetMathLibrary.MakeTransform` _output_get_5))
            (elif (`KismetStringLibrary.EqualEqual_StrStr` (`self.Next_Room_Picked`) "South")
              (bind _output_get_6 (set `self.Normal_Room_Picked` (`|GetArrayItem` _normal_rooms_north (`KismetMathLibrary.RandomIntegerInRange` 0 (- (`KismetArrayLibrary.Array_Length` _normal_rooms_north) 1)))))
              (`InstancedStaticMeshComponent.AddInstance` _output_get_6 (`KismetMathLibrary.MakeTransform` _lastcreatedtilelocation_2))
              (`KismetArrayLibrary.Array_Add` (`self.Created_Room_Location`) _lastcreatedtilelocation_2)
              (`KismetArrayLibrary.Array_RemoveItem` (`self.Available_Grid_Location`) _lastcreatedtilelocation_2)
              (`KismetArrayLibrary.Array_RemoveItem` (`self.Normal_Rooms_North`) _normal_room_picked :!label _label)
              (`KismetArrayLibrary.Array_RemoveItem` (`self.Normal_Rooms_South`) _normal_room_picked)
              (`KismetArrayLibrary.Array_RemoveItem` (`self.Normal_Rooms_East`) _normal_room_picked)
              (`KismetArrayLibrary.Array_RemoveItem` (`self.Normal_Rooms_West`) _normal_room_picked)
              (elif (`KismetStringLibrary.EqualEqual_StrStr` (`self.Next_Room_Picked`) "North")
                (bind _output_get_7 (set `self.Normal_Room_Picked` (`|GetArrayItem` _normal_rooms_south (`KismetMathLibrary.RandomIntegerInRange` 0 (- (`KismetArrayLibrary.Array_Length` _normal_rooms_south) 1)))))
                (`InstancedStaticMeshComponent.AddInstance` _output_get_7 (`KismetMathLibrary.MakeTransform` _lastcreatedtilelocation_3))
                (`KismetArrayLibrary.Array_Add` (`self.Created_Room_Location`) _lastcreatedtilelocation_3)
                (`KismetArrayLibrary.Array_RemoveItem` (`self.Available_Grid_Location`) _lastcreatedtilelocation_3)
                (goto _label)
                (elif (`KismetStringLibrary.EqualEqual_StrStr` (`self.Next_Room_Picked`) "West")
                  (bind _output_get_8 (set `self.Normal_Room_Picked` (`|GetArrayItem` _normal_rooms_east (`KismetMathLibrary.RandomIntegerInRange` 0 (- (`KismetArrayLibrary.Array_Length` _normal_rooms_east) 1)))))
                  (`InstancedStaticMeshComponent.AddInstance` _output_get_8 (`KismetMathLibrary.MakeTransform` _lastcreatedtilelocation_4))
                  (`KismetArrayLibrary.Array_Add` (`self.Created_Room_Location`) _lastcreatedtilelocation_4)
                  (`KismetArrayLibrary.Array_RemoveItem` (`self.Available_Grid_Location`) _lastcreatedtilelocation_4)
                  (goto _label)
                  (elif (`KismetStringLibrary.EqualEqual_StrStr` (`self.Next_Room_Picked`) "East")
                    (bind _output_get_9 (set `self.Normal_Room_Picked` (`|GetArrayItem` _normal_rooms_west (`KismetMathLibrary.RandomIntegerInRange` 0 (- (`KismetArrayLibrary.Array_Length` _normal_rooms_west) 1)))))
                    (`InstancedStaticMeshComponent.AddInstance` _output_get_9 (`KismetMathLibrary.MakeTransform` _lastcreatedtilelocation))
                    (`KismetArrayLibrary.Array_Add` (`self.Created_Room_Location`) _lastcreatedtilelocation)
                    (`KismetArrayLibrary.Array_RemoveItem` (`self.Available_Grid_Location`) _lastcreatedtilelocation)
                    (goto _label)))))))))))

(fn `Add_Room_Corridor_Infos`
  (params (Room :type "InstancedStaticMeshComponent Object Reference") (`Corridor Entry` :type "/Game/RogueLike_Game/Blueprints/Map_Generation/Room_Structure Structure"))
  (`BlueprintMapLibrary.Map_Add` (`self.Room_Corridor_Entry_Infos`) Room (make `/Game/RogueLike_Game/Blueprints/Map_Generation/Room_Structure` `Corridor Entry_North_2_E3B490C445E663D16B46B0A0D91C54BE` `Corridor Entry_South_3_DCC0241B446A85D924B11096E28BCDA3` `Corridor Entry_East_6_0F1263E84CFC3EB3BECD78A5634E4723` `Corridor Entry_West_7_556C14CE40AFF1CA6AF804ADD6AF37B6`)))

(fn `UserConstructionScript`)