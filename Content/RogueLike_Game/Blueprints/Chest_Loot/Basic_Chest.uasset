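; Basic loot chest for a roguelike that, when opened, rolls loot and spawns a Basic_Item with the chosen item name.
; Rarity, item type and armor type use percentage-threshold rolls, though every branch currently returns the same value, making item type always Gold.
; ChooseItem handles only Armor, picking randomly among ArmorDataTable rows of the rolled type.
; Rarity is passed in but unused, and Gold yields no item selection.
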(event `Open_Chest`
  (bind _rarity_output (`self.Choose_Rarity` 0))
  (bind _loottype_output (`self.Choose_ItemType` 0))
  (bind _item_name (`self.Choose_Item` _loottype_output _rarity_output))
  (`|SpawnActorFromClass` "/Game/RogueLike_Game/Blueprints/Chest_Loot/Basic_Item.Basic_Item_C" (`KismetMathLibrary.MakeTransform` (0.0 0.0 0.0)) "Undefined" "OverrideRootScale" null _item_name null))

(fn `Choose_ArmorType`
  (params (LootChance_Modifier :type Integer))
  (returns (ArmorType_Output :type "/Game/RogueLike_Game/Blueprints/Chest_Loot/TypeOfArmor Enum"))
  (locals (Random_Int :type Integer :default 0))
  (bind _output_get (set `local.Random_Int` (`KismetMathLibrary.RandomIntegerInRange` 1 100)))
  (if (<= _output_get (- 40 LootChance_Modifier))
    (return "NewEnumerator0")
    (elif (<= (`local.Random_Int`) (- 70 LootChance_Modifier))
      (return "NewEnumerator0")
      (elif (<= (`local.Random_Int`) (- 90 LootChance_Modifier))
        (return "NewEnumerator0")
        (else
          (return "NewEnumerator0"))))))

(fn `Choose_Item`
  (params (ItemType :type "/Game/RogueLike_Game/Blueprints/Chest_Loot/LootType_Enum Enum" :default "NewEnumerator0") (Rarity :type Byte :default 0))
  (returns (Item_Name :type Name))
  (locals (Compatible_Items :type "Array of Name"))
  (bind _compatible_items (`local.Compatible_Items`))
  (switch `/Game/RogueLike_Game/Blueprints/Chest_Loot/LootType_Enum` ItemType
    (:`NewEnumerator2`
      (bind _armortype_output (`self.Choose_ArmorType` 0))
      (bind _outrownames (`DataTableFunctionLibrary.GetDataTableRowNames` "/Game/RogueLike_Game/Blueprints/Chest_Loot/ArmorDataTable.ArmorDataTable"))
      (for _array_element _outrownames
        (bind _returnvalue (`|GetDataTableRow` "/Game/RogueLike_Game/Blueprints/Chest_Loot/ArmorDataTable.ArmorDataTable" _array_element)
          (:`then`
            (bind (_name _rarity _armor _typeofarmor) (break `/Game/RogueLike_Game/Blueprints/Chest_Loot/Armor_Data_Structure` _returnvalue))
            (if (`|EnumEquality` _typeofarmor _armortype_output)
              (`KismetArrayLibrary.Array_Add` (`local.Compatible_Items`) _name)))))
      (return (`|GetArrayItem` _compatible_items (`KismetMathLibrary.RandomIntegerInRange` 0 (`KismetArrayLibrary.Array_LastIndex` _compatible_items)))))))

(fn `Choose_ItemType`
  (params (LootChance_Modifier :type Integer))
  (returns (LootType_Output :type "/Game/RogueLike_Game/Blueprints/Chest_Loot/LootType_Enum Enum"))
  (locals (Random_Int :type Integer :default 0))
  (bind _output_get (set `local.Random_Int` (`KismetMathLibrary.RandomIntegerInRange` 1 100)))
  (if (<= _output_get (- 40 LootChance_Modifier))
    (return "NewEnumerator0")
    (elif (<= (`local.Random_Int`) (- 70 LootChance_Modifier))
      (return "NewEnumerator0")
      (elif (<= (`local.Random_Int`) (- 90 LootChance_Modifier))
        (return "NewEnumerator0")
        (else
          (return "NewEnumerator0"))))))

(fn `Choose_Rarity`
  (params (LootChance_Modifier :type Integer))
  (returns (Rarity_Output :type "/Game/RogueLike_Game/Blueprints/Loot/Rarity_Enum Enum"))
  (locals (Random_Int :type Integer :default 0))
  (bind _output_get (set `local.Random_Int` (`KismetMathLibrary.RandomIntegerInRange` 1 100)))
  (if (<= _output_get (- 40 LootChance_Modifier))
    (return "NewEnumerator0")
    (elif (<= (`local.Random_Int`) (- 70 LootChance_Modifier))
      (return "NewEnumerator0")
      (elif (<= (`local.Random_Int`) (- 90 LootChance_Modifier))
        (return "NewEnumerator0")
        (else
          (return "NewEnumerator0"))))))

(fn `UserConstructionScript`)