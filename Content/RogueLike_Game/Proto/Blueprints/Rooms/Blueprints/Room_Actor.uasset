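; Roguelike room actor that spawns doors on its flagged N/E/S/W sides and shows its own icon on the minimap.
; The Construction Script adds door child actors at per-side transforms and positions the collision box.
; BeginPlay concatenates the door flags into a direction string that keys a texture map for the icon.
; The icon starts hidden, then appears with an animation for the entry room, on player overlap, or through ShowMiniMapRoom.
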(event `self.ReceiveBeginPlay`
  (bind _minimap_room_widget (`self.MiniMap_Room_Widget`))
  (bind _returnvalue (`WidgetComponent.GetUserWidgetObject` _minimap_room_widget))
  (`|ExecutionSequence`
    (:`then_0`
      (`SceneComponent.SetVisibility` (`self.MiniMap_Room_Widget`) false false)
      (if (`self.Entry_Room?`)
        (`/Engine/EditorBlueprintResources/StandardMacros.DoOnce` false
          (:`Completed`
            (`SceneComponent.SetVisibility` _minimap_room_widget true false)
            (bind _asmini_map_room_widget (cast `/Game/RogueLike_Game/Proto/Blueprints/Rooms/Widget/MiniMap_Room_Widget` _returnvalue))
            (`UserWidget.PlayAnimation` _returnvalue (`/Game/RogueLike_Game/Proto/Blueprints/Rooms/Widget/MiniMap_Room_Widget.Room_Logo_Animation` _asmini_map_room_widget) 0.0 1 "Forward" 1.0 false)))))
    (:`then_1`
      (`self.Set_Room_Directions` (`self.Door_N`) "N")
      (`self.Set_Room_Directions` (`self.Door_E`) "E")
      (`self.Set_Room_Directions` (`self.Door_S`) "S")
      (`self.Set_Room_Directions` (`self.Door_W`) "W"))
    (:`then_2`
      (bind _asmini_map_room_widget_2 (cast `/Game/RogueLike_Game/Proto/Blueprints/Rooms/Widget/MiniMap_Room_Widget` (`WidgetComponent.GetUserWidgetObject` (`self.MiniMap_Room_Widget`))))
      (`Image.SetBrush` (`/Game/RogueLike_Game/Proto/Blueprints/Rooms/Widget/MiniMap_Room_Widget.Room_Logo` _asmini_map_room_widget_2) (make `SlateBrush` (32.0 32.0) (struct) (struct :`SpecifiedColor` (struct :`R` 1.0 :`G` 1.0 :`B` 1.0 :`A` 1.0) :`ColorUseRule` "UseColor_Specified") (`BlueprintMapLibrary.Map_Find` (`self.MiniMap_Room_Texture`) (`self.Room_Directions`)))))))

(event `self.Box_Collision.OnComponentBeginOverlap`
  (params (OverlappedComponent :type "PrimitiveComponent Object Reference") (OtherActor :type "Actor Object Reference") (OtherComp :type "PrimitiveComponent Object Reference") (OtherBodyIndex :type Integer) (bFromSweep :type Boolean) (SweepResult :type "HitResult Structure (by ref)"))
  (bind _minimap_room_widget (`self.MiniMap_Room_Widget`))
  (bind _returnvalue (`WidgetComponent.GetUserWidgetObject` _minimap_room_widget))
  (if (`self.ActorHasTag` OtherActor "PlayerCharacter")
    (`/Engine/EditorBlueprintResources/StandardMacros.DoOnce` false
      (:`Completed`
        (`SceneComponent.SetVisibility` _minimap_room_widget true false)
        (bind _asmini_map_room_widget (cast `/Game/RogueLike_Game/Proto/Blueprints/Rooms/Widget/MiniMap_Room_Widget` _returnvalue))
        (`UserWidget.PlayAnimation` _returnvalue (`/Game/RogueLike_Game/Proto/Blueprints/Rooms/Widget/MiniMap_Room_Widget.Room_Logo_Animation` _asmini_map_room_widget) 0.0 1 "Forward" 1.0 false)))))

(fn `Set_Room_Directions`
  (params (Condition :type Boolean) (String :type String))
  (if Condition
    (set `self.Room_Directions` (`KismetStringLibrary.Concat_StrStr` (`self.Room_Directions`) String))))

(fn `Show_MiniMap_Room`
  (bind _minimap_room_widget (`self.MiniMap_Room_Widget`))
  (bind _returnvalue (`WidgetComponent.GetUserWidgetObject` _minimap_room_widget))
  (`/Engine/EditorBlueprintResources/StandardMacros.DoOnce` false
    (:`Completed`
      (`SceneComponent.SetVisibility` _minimap_room_widget true false)
      (bind _asmini_map_room_widget (cast `/Game/RogueLike_Game/Proto/Blueprints/Rooms/Widget/MiniMap_Room_Widget` _returnvalue))
      (`UserWidget.PlayAnimation` _returnvalue (`/Game/RogueLike_Game/Proto/Blueprints/Rooms/Widget/MiniMap_Room_Widget.Room_Logo_Animation` _asmini_map_room_widget) 0.0 1 "Forward" 1.0 false))))

(fn `Spawning_Door`
  (`|ExecutionSequence`
    (:`then_0`
      (if (`self.Door_N`)
        (`AddComponent|NODE_AddChildActorComponent-1` :`RelativeTransform` (`self.Door_N_Transform`))))
    (:`then_1`
      (if (`self.Door_S`)
        (`AddComponent|NODE_AddChildActorComponent-2` :`RelativeTransform` (`self.Door_S_Transform`))))
    (:`then_2`
      (if (`self.Door_W`)
        (`AddComponent|NODE_AddChildActorComponent-3` :`RelativeTransform` (`self.Door_W_Transform`))))
    (:`then_3`
      (if (`self.Door_E`)
        (`AddComponent|NODE_AddChildActorComponent-4` :`RelativeTransform` (`self.Door_E_Transform`))))))

(fn `UserConstructionScript`
  (`|ExecutionSequence`
    (:`then_0`
      (`self.Spawning_Door`))
    (:`then_1`
      (`SceneComponent.K2_SetRelativeTransform` (`self.Box_Collision`) (`self.Collision_Box_Transform`) false false))))