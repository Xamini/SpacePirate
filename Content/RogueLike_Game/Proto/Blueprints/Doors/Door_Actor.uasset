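; Roguelike door actor that slides open once when the player enters its collision box, unless it is locked.
; On start, it takes lock state and level from its parent Room_Actor for one room type, showing and collecting the matching lock meshes.
; A capsule overlap highlights locks via custom depth and enables interaction, polled on Tick.
; Each interaction spends a ChestKey to remove one lock; removing the last opens the door.
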(event `self.ReceiveBeginPlay`
  (`KismetSystemLibrary.Delay` 0.2)
  (`|ExecutionSequence`
    (:`then_0`
      (bind _asroom_actor (cast `/Game/RogueLike_Game/Proto/Blueprints/Rooms/Blueprints/Room_Actor` (`self.GetParentActor`)))
      (if (`|EnumEquality` (`/Game/RogueLike_Game/Proto/Blueprints/Rooms/Blueprints/Room_Actor.Room_Type` _asroom_actor) "NewEnumerator6")
        (set `self.Locked?` true)
        (set `self.Locked_Level` (`/Game/RogueLike_Game/Proto/Blueprints/Rooms/Blueprints/Room_Actor.Locked_Level` _asroom_actor))))
    (:`then_1`
      (if (`self.Locked?`)
        (if (== (`self.Locked_Level`) 1)
          (`SceneComponent.SetVisibility` (`self.1_Lock`) true true)
          (elif (== (`self.Locked_Level`) 2)
            (`SceneComponent.SetVisibility` (`self.2_Locks`) true true)
            (elif (== (`self.Locked_Level`) 3)
              (`SceneComponent.SetVisibility` (`self.3_Locks`) true true))))))
    (:`then_2`
      (for _array_element (`|MakeArray` (`self.Lock_1_01`) (`self.Lock_2_01`) (`self.Lock_2_02`) (`self.Lock_3_01`) (`self.Lock_3_02`) (`self.Lock_3_03`))
        (if (`KismetStringLibrary.Contains` (`KismetSystemLibrary.GetObjectName` _array_element) (`KismetStringLibrary.Concat_StrStr` "Lock_" (`KismetStringLibrary.Conv_IntToString` (`self.Locked_Level`))))
          (`KismetArrayLibrary.Array_Add` (`self.Locks_Array`) _array_element))))))

(event `self.Collision_Box.OnComponentBeginOverlap`
  (params (OverlappedComponent :type "PrimitiveComponent Object Reference") (OtherActor :type "Actor Object Reference") (OtherComp :type "PrimitiveComponent Object Reference") (OtherBodyIndex :type Integer) (bFromSweep :type Boolean) (SweepResult :type "HitResult Structure (by ref)"))
  (if (`self.ActorHasTag` OtherActor "PlayerCharacter")
    (if (not (`self.Locked?`))
      (`/Engine/EditorBlueprintResources/StandardMacros.DoOnce` false :!label _label
        (:`Completed`
          (set `self.Current_Location` (`SceneComponent.RelativeLocation` (`self.Door_Mesh`)))
          (bind (_direction _lerp_value) (`Timeline|Opening_Door` :!via `PlayFromStart`)
            (:`Update`
              (`SceneComponent.K2_SetRelativeLocation` (`self.Door_Mesh`) (`KismetMathLibrary.VLerp` (`self.Current_Location`) (`self.Open_Location`) _lerp_value) false false))))))))

(event `Open_Door_After_Unlock`
  (goto _label))

(event `self.Capsule.OnComponentBeginOverlap`
  (params (OverlappedComponent :type "PrimitiveComponent Object Reference") (OtherActor :type "Actor Object Reference") (OtherComp :type "PrimitiveComponent Object Reference") (OtherBodyIndex :type Integer) (bFromSweep :type Boolean) (SweepResult :type "HitResult Structure (by ref)"))
  (if (`self.Locked?`)
    (for _array_element (`self.Locks_Array`)
      (`PrimitiveComponent.SetRenderCustomDepth` _array_element true))
    (set `self.Player_Can_Interact` true)))

(event `self.Capsule.OnComponentEndOverlap`
  (params (OverlappedComponent :type "PrimitiveComponent Object Reference") (OtherActor :type "Actor Object Reference") (OtherComp :type "PrimitiveComponent Object Reference") (OtherBodyIndex :type Integer))
  (for _array_element (`self.Locks_Array`)
    (`PrimitiveComponent.SetRenderCustomDepth` _array_element false))
  (set `self.Player_Can_Interact` false))

(event `self.ReceiveTick`
  (params (DeltaSeconds :type "Float (single-precision)"))
  (bind _locks_array (`self.Locks_Array`))
  (bind _output (`|GetArrayItem` _locks_array))
  (bind _asplayer_character (cast `/Game/RogueLike_Game/Proto/Characters/Player/Blueprints/Player_Character` (`GameplayStatics.GetPlayerCharacter` 0)))
  (if (`self.Player_Can_Interact`)
    (if (`/Game/RogueLike_Game/Proto/Characters/Player/Blueprints/Player_Character.Interact?` _asplayer_character)
      (bind _asplayer_character_2 (cast `/Game/RogueLike_Game/Proto/Characters/Player/Blueprints/Player_Character` (`GameplayStatics.GetPlayerCharacter` 0)))
      (if (> (`/Game/RogueLike_Game/Proto/Characters/Player/Blueprints/Player_Character.Chest_Keys` _asplayer_character_2) 0)
        (set `/Game/RogueLike_Game/Proto/Characters/Player/Blueprints/Player_Character.Chest_Keys` (- (`/Game/RogueLike_Game/Proto/Characters/Player/Blueprints/Player_Character.Chest_Keys` _asplayer_character_2) 1) _asplayer_character_2)
        (set `/Game/RogueLike_Game/Proto/Characters/Player/Blueprints/Player_Character.Interact?` false _asplayer_character_2)
        (`SceneComponent.SetVisibility` _output false false)
        (`KismetArrayLibrary.Array_RemoveItem` _locks_array _output)
        (if (== (`KismetArrayLibrary.Array_Length` _locks_array) 0)
          (set `self.Locked?` false)
          (`self.Open_Door_After_Unlock`))))))

(fn `UserConstructionScript`)