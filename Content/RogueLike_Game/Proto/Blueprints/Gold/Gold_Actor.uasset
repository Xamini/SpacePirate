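; Gold pickup actor that adds its Amount to the Player_Character's Gold and destroys itself on touching the player capsule.
; On BeginPlay it tints its mesh through a dynamic material and plays a timeline moving it to LocationAfterAnimation with a separate height curve.
; Overlapping a component tagged Gold_Attraction_Box starts a second timeline that lerps the gold toward the player's current position.
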(event `self.ReceiveBeginPlay`
  (bind _location_after_animation (`self.Location_After_Animation`))
  (bind _returnvalue (`PrimitiveComponent.CreateDynamicMaterialInstance` (`self.Gold`) 0 "/Game/RogueLike_Game/Proto/Blueprints/Gold/Gold_Material_Inst.Gold_Material_Inst" "None"))
  (`MaterialInstanceDynamic.SetVectorParameterValue` _returnvalue "Money_Color" (`self.Color`))
  (set `self.Spawn_Location` (`SceneComponent.K2_GetComponentLocation` (`self.DefaultSceneRoot`)))
  (bind (_direction _tz _lerp) (`Timeline|Spawn_Animation`)
    (:`Update`
      (bind (_returnvalue_x _returnvalue_y) (`KismetMathLibrary.BreakVector` (`KismetMathLibrary.VLerp` (`self.Spawn_Location`) _location_after_animation _lerp)))
      (`SceneComponent.K2_SetWorldLocation` (`self.DefaultSceneRoot`) (`KismetMathLibrary.MakeVector` _returnvalue_x _returnvalue_y (+ _tz (.z _location_after_animation))) false false))))

(event `self.Gold.OnComponentBeginOverlap`
  (params (OverlappedComponent :type "PrimitiveComponent Object Reference") (OtherActor :type "Actor Object Reference") (OtherComp :type "PrimitiveComponent Object Reference") (OtherBodyIndex :type Integer) (bFromSweep :type Boolean) (SweepResult :type "HitResult Structure (by ref)"))
  (if (`ActorComponent.ComponentHasTag` OtherComp "Gold_Attraction_Box")
    (bind (_direction _lerp) (`Timeline|Gold_Attraction_Timeline` :!via `PlayFromStart`)
      (:`Update`
        (`SceneComponent.K2_SetWorldLocation` (`self.DefaultSceneRoot`) (`KismetMathLibrary.VLerp` (`self.K2_GetActorLocation`) (`self.K2_GetActorLocation` (`GameplayStatics.GetPlayerCharacter` 0)) _lerp) false false)))
    (elif (`ActorComponent.ComponentHasTag` OtherComp "Player_Capsule")
      (bind _asplayer_character (cast `/Game/RogueLike_Game/Proto/Characters/Player/Blueprints/Player_Character` (`GameplayStatics.GetPlayerCharacter` 0)))
      (set `/Game/RogueLike_Game/Proto/Characters/Player/Blueprints/Player_Character.Gold` (+ (`/Game/RogueLike_Game/Proto/Characters/Player/Blueprints/Player_Character.Gold` _asplayer_character) (`self.Amount`)) _asplayer_character)
      (`self.K2_DestroyActor`))))

(fn `UserConstructionScript`)