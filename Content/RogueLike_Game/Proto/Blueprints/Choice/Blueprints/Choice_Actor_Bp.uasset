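; Roguelike loot choice actor that offers two loot items side by side and lets only one remain claimable.
; BeginPlay rolls a shared rarity from stage-percent thresholds (fixed key 3) and spawns two Loot_System_Actor_Proto child actors.
; Both get the same item type, currently hardcoded because the random type pick's result is unused.
; Tick polls the children while the choice is available; when one disappears, it destroys the other and closes the choice.
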(event `self.ReceiveBeginPlay`
  (`|ExecutionSequence`
    (:`then_0`
      (bind _rarity (`self.Pick Rarity`))
      (set `self.Rarity` _rarity)
      (`self.Pick Item Type`)
      (set `self.Item_Type` "NewEnumerator8"))
    (:`then_1`
      (for _index (range 2)
        (bind _returnvalue (`AddComponent|NODE_AddChildActorComponent-2` :`RelativeTransform` (`KismetMathLibrary.MakeTransform` (`KismetMathLibrary.MakeVector` (`BlueprintMapLibrary.Map_Find` (`self.Child_Actor_Location_X`) _index) 100.0))))
        (`KismetArrayLibrary.Array_Add` (`self.Child_Actor_List`) _returnvalue)
        (`ChildActorComponent.SetChildActorClass` _returnvalue "/Game/RogueLike_Game/Proto/Blueprints/Loot_System/Actor/Loot_System_Actor_Proto.Loot_System_Actor_Proto_C")
        (bind _asloot_system_actor_proto (cast `/Game/RogueLike_Game/Proto/Blueprints/Loot_System/Actor/Loot_System_Actor_Proto` (`ChildActorComponent.ChildActor` _returnvalue)))
        (set `/Game/RogueLike_Game/Proto/Blueprints/Loot_System/Actor/Loot_System_Actor_Proto.Loot_System_Type` "NewEnumerator1" _asloot_system_actor_proto)
        (set `/Game/RogueLike_Game/Proto/Blueprints/Loot_System/Actor/Loot_System_Actor_Proto.Item_Rarity` (`self.Rarity`) _asloot_system_actor_proto)
        (set `/Game/RogueLike_Game/Proto/Blueprints/Loot_System/Actor/Loot_System_Actor_Proto.Item_Type` (`self.Item_Type`) _asloot_system_actor_proto)))))

(event `self.ReceiveTick`
  (params (DeltaSeconds :type "Float (single-precision)"))
  (if (`self.Choice_Available?`)
    (for (_array_element _array_index) (`self.Child_Actor_List`)
      (`/Engine/EditorBlueprintResources/StandardMacros.IsValid` (`ChildActorComponent.ChildActor` _array_element)
        (:`Is Not Valid`
          (`KismetArrayLibrary.Array_Remove` (`self.Child_Actor_List`) _array_index)
          (`self.K2_DestroyActor` (`ChildActorComponent.ChildActor` (`|GetArrayItem` (`self.Child_Actor_List`))))
          (set `self.Choice_Available?` false))))))

(fn `Pick Item Type`
  (returns (Item_Type :type "/Game/RogueLike_Game/Proto/Blueprints/Loot_System/Actor/Utilities/Enum/Item_Type_Enum Enum"))
  (return (select `int` (`KismetMathLibrary.RandomIntegerInRange` 0 2) :`0` "NewEnumerator7" :`1` "NewEnumerator8" :`2` "NewEnumerator9" :!type "/Game/RogueLike_Game/Proto/Blueprints/Loot_System/Actor/Utilities/Enum/Item_Type_Enum Enum")))

(fn `Pick Rarity`
  (returns (Rarity :type "/Game/RogueLike_Game/Proto/Blueprints/Loot_System/Actor/Utilities/Enum/Rarity_Enum Enum"))
  (locals (Percent :type Integer) (Stage_Percent :type "Map of Integer to Integer"))
  (bind _value (`BlueprintMapLibrary.Map_Find` (`local.Stage_Percent`) 3))
  (bind _output_get (set `local.Percent` (`KismetMathLibrary.RandomIntegerInRange` 1 100)))
  (if (<= _output_get (+ 0 _value))
    (return "NewEnumerator2")
    (elif (<= (`local.Percent`) (+ 30 _value))
      (return "NewEnumerator1")
      (else
        (return "NewEnumerator0")))))

(fn `UserConstructionScript`)