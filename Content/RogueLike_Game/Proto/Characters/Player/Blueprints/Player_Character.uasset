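; Player character Blueprint for a roguelike: diagonal-axis movement that turns to face the cursor, an interact flag, and inventory and map menu toggles.
; While the map is open, input pans, zooms and recenters the MapMenu_Camera_Actor orthographic capture, scaling pan by zoom.
; Map teleport moves the capsule to that actor's hit component behind a brief HUD.
; Update_Statistics derives stats from PlayerStatsMap, which Tick prints every frame.
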(event `Teleport_From_Map`
  ;[1 1 1] Map_Teleportation
  (`Widget.RemoveFromParent` (`self.MapMenu_Widget`))
  (set `self.MapMenu Open?` false)
  (`|ExecutionSequence`
    (:`then_0`
      (`KismetSystemLibrary.Delay` 0.1)
      (bind _returnvalue (`|CreateWidget` "/Game/RogueLike_Game/Proto/Characters/Player/Widgets/Teleport_HUD.Teleport_HUD_C"))
      (`UserWidget.AddToViewport` _returnvalue 0)
      (`KismetSystemLibrary.Delay` 0.75)
      (`Widget.RemoveFromParent` _returnvalue))
    (:`then_1`
      (`KismetSystemLibrary.Delay` 0.2)
      (bind _outactors (`GameplayStatics.GetAllActorsOfClass` "/Game/RogueLike_Game/Proto/Characters/Player/Widgets/MapMenu/Blueprints/MapMenu_Camera_Actor.MapMenu_Camera_Actor_C"))
      (bind _output (`|GetArrayItem` _outactors))
      (bind _current_hit_component (`/Game/RogueLike_Game/Proto/Characters/Player/Widgets/MapMenu/Blueprints/MapMenu_Camera_Actor.Current_Hit_Component` _output))
      (`PrimitiveComponent.SetCustomDepthStencilValue` _current_hit_component (`/Game/RogueLike_Game/Proto/Characters/Player/Widgets/MapMenu/Blueprints/MapMenu_Camera_Actor.Current_Stencil_Value_Component` _output))
      (bind (_returnvalue_x _returnvalue_y) (`KismetMathLibrary.BreakVector` (`SceneComponent.K2_GetComponentLocation` _current_hit_component)))
      (`SceneComponent.K2_SetWorldLocation` (`self.CapsuleComponent`) (`KismetMathLibrary.MakeVector` _returnvalue_x _returnvalue_y 95.0) false false))))

(event `InputAxis|LeftClick_Hold`
  (params (AxisValue :type "Float (single-precision)"))
  (bind _returnvalue (`self.GetInputAxisKeyValue`))
  (bind _returnvalue_2 (`self.GetInputAxisKeyValue`))
  ;[1 1 1] Drag MapMenu
  (if (`self.MapMenu Open?`)
    (bind _outactors (`GameplayStatics.GetAllActorsOfClass` "/Game/RogueLike_Game/Proto/Characters/Player/Widgets/MapMenu/Blueprints/MapMenu_Camera_Actor.MapMenu_Camera_Actor_C"))
    (if (> _returnvalue 0.0)
      (bind _output (`|GetArrayItem` _outactors))
      (bind _defaultsceneroot (`/Game/RogueLike_Game/Proto/Characters/Player/Widgets/MapMenu/Blueprints/MapMenu_Camera_Actor.DefaultSceneRoot` _output))
      (bind (_returnvalue_x _returnvalue_y) (`KismetMathLibrary.BreakVector` (`SceneComponent.K2_GetComponentLocation` _defaultsceneroot)))
      (bind _returnvalue_3 (* (/ (`SceneCaptureComponent2D.OrthoWidth` (`/Game/RogueLike_Game/Proto/Characters/Player/Widgets/MapMenu/Blueprints/MapMenu_Camera_Actor.MapMenu_ComponentCapture` _output)) 100.0) (* (`KismetMathLibrary.Abs` _returnvalue) -1.0)))
      (`SceneComponent.K2_SetWorldLocation` _defaultsceneroot (`KismetMathLibrary.MakeVector` (+ _returnvalue_x _returnvalue_3) (+ _returnvalue_y _returnvalue_3) -1000.0) false false)
      (elif (< _returnvalue 0.0)
        (`SceneComponent.K2_SetWorldLocation` _defaultsceneroot (`KismetMathLibrary.MakeVector` (- _returnvalue_x _returnvalue_3) (- _returnvalue_y _returnvalue_3) -1000.0) false false)))
    (if (< _returnvalue_2 0.0)
      (bind _defaultsceneroot_2 (`/Game/RogueLike_Game/Proto/Characters/Player/Widgets/MapMenu/Blueprints/MapMenu_Camera_Actor.DefaultSceneRoot` _output))
      (bind (_returnvalue_x_2 _returnvalue_y_2) (`KismetMathLibrary.BreakVector` (`SceneComponent.K2_GetComponentLocation` _defaultsceneroot_2)))
      (bind _returnvalue_4 (* (/ (`SceneCaptureComponent2D.OrthoWidth` (`/Game/RogueLike_Game/Proto/Characters/Player/Widgets/MapMenu/Blueprints/MapMenu_Camera_Actor.MapMenu_ComponentCapture` _output)) 100.0) (`KismetMathLibrary.Abs` _returnvalue_2)))
      (`SceneComponent.K2_SetWorldLocation` _defaultsceneroot_2 (`KismetMathLibrary.MakeVector` (- _returnvalue_x_2 _returnvalue_4) (+ _returnvalue_y_2 _returnvalue_4) -1000.0) false false)
      (elif (> _returnvalue_2 0.0)
        (`SceneComponent.K2_SetWorldLocation` _defaultsceneroot_2 (`KismetMathLibrary.MakeVector` (+ _returnvalue_x_2 _returnvalue_4) (- _returnvalue_y_2 _returnvalue_4) -1000.0) false false)))))

(event `Key|MouseScrollUp`
  (params (Key :type "Key Structure"))
  ;[1 1 1] Zoom In/Out MapMenu
  (:`Pressed`
    (if (`self.MapMenu Open?`) :!label _label
      (bind _returnvalue (`GameplayStatics.GetActorOfClass` "/Game/RogueLike_Game/Proto/Characters/Player/Widgets/MapMenu/Blueprints/MapMenu_Camera_Actor.MapMenu_Camera_Actor_C"))
      (bind _mapmenu_componentcapture (`/Game/RogueLike_Game/Proto/Characters/Player/Widgets/MapMenu/Blueprints/MapMenu_Camera_Actor.MapMenu_ComponentCapture` _returnvalue))
      (bind _orthowidth (`SceneCaptureComponent2D.OrthoWidth` _mapmenu_componentcapture))
      (if (> _orthowidth (`self.Min_MapMenu_Zoom`))
        (set `SceneCaptureComponent2D.OrthoWidth` (- _orthowidth 5000.0) _mapmenu_componentcapture)))))

(event `InputAxisKey|Gamepad_RightTriggerAxis`
  (params (AxisValue :type "Float (single-precision)"))
  ;[1 1 1] Zoom In/Out MapMenu
  (if (> AxisValue 0.0)
    (goto _label)))

(event `Key|MouseScrollDown`
  (params (Key :type "Key Structure"))
  ;[1 1 1] Zoom In/Out MapMenu
  (:`Pressed`
    (if (`self.MapMenu Open?`) :!label _label_2
      (bind _returnvalue (`GameplayStatics.GetActorOfClass` "/Game/RogueLike_Game/Proto/Characters/Player/Widgets/MapMenu/Blueprints/MapMenu_Camera_Actor.MapMenu_Camera_Actor_C"))
      (bind _mapmenu_componentcapture (`/Game/RogueLike_Game/Proto/Characters/Player/Widgets/MapMenu/Blueprints/MapMenu_Camera_Actor.MapMenu_ComponentCapture` _returnvalue))
      (bind _orthowidth (`SceneCaptureComponent2D.OrthoWidth` _mapmenu_componentcapture))
      (if (< _orthowidth (`self.Max_MapMenu_Zoom`))
        (set `SceneCaptureComponent2D.OrthoWidth` (+ _orthowidth 5000.0) _mapmenu_componentcapture)))))

(event `InputAxisKey|Gamepad_LeftTriggerAxis`
  (params (AxisValue :type "Float (single-precision)"))
  ;[1 1 1] Zoom In/Out MapMenu
  (if (> AxisValue 0.0)
    (goto _label_2)))

(event `InputAction|Recenter_Map_Menu`
  (params (Key :type "Key Structure"))
  (bind (_returnvalue_x _returnvalue_y) (`KismetMathLibrary.BreakVector` (`self.K2_GetActorLocation`)))
  ;[1 1 1] Recenter_MapMenu
  (:`Pressed`
    (if (`self.MapMenu Open?`)
      (bind _outactors (`GameplayStatics.GetAllActorsOfClass` "/Game/RogueLike_Game/Proto/Characters/Player/Widgets/MapMenu/Blueprints/MapMenu_Camera_Actor.MapMenu_Camera_Actor_C"))
      (`SceneComponent.K2_SetWorldLocation` (`/Game/RogueLike_Game/Proto/Characters/Player/Widgets/MapMenu/Blueprints/MapMenu_Camera_Actor.DefaultSceneRoot` (`|GetArrayItem` _outactors)) (`KismetMathLibrary.MakeVector` _returnvalue_x _returnvalue_y -1000.0) false false))))

(event `InputAction|Open_MapMenu`
  (params (Key :type "Key Structure"))
  (bind (_returnvalue_x _returnvalue_y) (`KismetMathLibrary.BreakVector` (`self.K2_GetActorLocation`)))
  ;[1 1 1] Open_Map
  (:`Pressed`
    (if (`self.Is in HUB?`)
      _
      (elif (`self.MapMenu Open?`)
        (`Widget.RemoveFromParent` (`self.MapMenu_Widget`) :!label _label_3)
        (set `self.MapMenu Open?` false)
        (else
          (bind _returnvalue (`|CreateWidget` "/Game/RogueLike_Game/Proto/Characters/Player/Widgets/MapMenu/Widgets/MapMenu_Widget.MapMenu_Widget_C"))
          (bind _output_get (set `self.MapMenu_Widget` _returnvalue))
          (`UserWidget.AddToViewport` _output_get 0)
          (set `self.MapMenu Open?` true)
          (bind _returnvalue_2 (`GameplayStatics.GetActorOfClass` "/Game/RogueLike_Game/Proto/Characters/Player/Widgets/MapMenu/Blueprints/MapMenu_Camera_Actor.MapMenu_Camera_Actor_C"))
          (`SceneComponent.K2_SetWorldLocation` (`/Game/RogueLike_Game/Proto/Characters/Player/Widgets/MapMenu/Blueprints/MapMenu_Camera_Actor.DefaultSceneRoot` _returnvalue_2) (`KismetMathLibrary.MakeVector` _returnvalue_x _returnvalue_y -1000.0) false false))))))

(event `Key|Gamepad_FaceButton_Right`
  (params (Key :type "Key Structure"))
  ;[1 1 1] Open_Map
  (:`Pressed`
    (if (`self.MapMenu Open?`)
      (goto _label_3))))

(event `InputAction|Inventory_Menu`
  (params (Key :type "Key Structure"))
  ;[1 1 1] Open_Inventory
  (:`Pressed`
    (if (`self.Inventory_Open?`)
      (`Widget.RemoveFromParent` (stale _returnvalue))
      (set `self.Inventory_Open?` false)
      (else
        (bind _returnvalue (`|CreateWidget` "/Game/RogueLike_Game/Proto/Characters/Player/Widgets/Inventaire/Inventory_Widget.Inventory_Widget_C"))
        (`UserWidget.AddToViewport` _returnvalue 0)
        (set `self.Inventory_Open?` true)))))

(event `InputAction|Interaction`
  (params (Key :type "Key Structure"))
  ;[1 1 1] Interact
  (:`Pressed`
    (set `self.Interact?` true))
  (:`Released`
    (set `self.Interact?` false)))

(event `InputAxis|MoveForward`
  (params (AxisValue :type "Float (single-precision)"))
  (bind _returnvalue (* AxisValue 100.0))
  ;[1 1 1] Player Movement
  (if (`self.Can_Move?`)
    (if (`self.MapMenu Open?`)
      (`self.Move Map Menu XAxis` AxisValue)
      (else
        (`self.AddMovementInput` (`KismetMathLibrary.MakeVector` _returnvalue _returnvalue))
        (`self.Character_Look_At_Cursor` :!label _label_4)))))

(event `InputAxis|MoveRight`
  (params (AxisValue :type "Float (single-precision)"))
  (bind _returnvalue (* AxisValue 100.0))
  ;[1 1 1] Player Movement
  (if (`self.Can_Move?`)
    (if (`self.MapMenu Open?`)
      (`self.Move Map Menu YAxis` AxisValue)
      (else
        (`self.AddMovementInput` (`KismetMathLibrary.MakeVector` (* _returnvalue -1.0) _returnvalue))
        (goto _label_4)))))

(event `Update_Statistics`
  (bind _returnvalue (* (`BlueprintMapLibrary.Map_Find` (`self.Player_Stats_Map`) "NewEnumerator6") 2))
  ;[1 1 1] Update Stats
  (bind _keys (`BlueprintMapLibrary.Map_Keys` (`self.Player_Stats_Map`)))
  (for _array_element _keys
    (switch `/Game/RogueLike_Game/Proto/Blueprints/Loot_System/Actor/Utilities/Enum/Statistics_Type` _array_element
      (:`NewEnumerator0`
        (set `CharacterMovementComponent.MaxWalkSpeed` (`KismetMathLibrary.Conv_IntToDouble` (+ (* (`BlueprintMapLibrary.Map_Find` (`self.Player_Stats_Map`) "NewEnumerator0") 20) 600)) (`self.CharacterMovement`)))
      (:`NewEnumerator3`
        (set `self.Resistance` (`KismetMathLibrary.Conv_IntToDouble` (* (`BlueprintMapLibrary.Map_Find` (`self.Player_Stats_Map`) "NewEnumerator3") 2))))
      (:`NewEnumerator4`
        (set `self.Max_Vitality` (+ (* (`BlueprintMapLibrary.Map_Find` (`self.Player_Stats_Map`) "NewEnumerator4") 5) 100)))
      (:`NewEnumerator5`
        (set `self.Dexterity` (`KismetMathLibrary.Conv_IntToDouble` (* (`BlueprintMapLibrary.Map_Find` (`self.Player_Stats_Map`) "NewEnumerator5") 2))))
      (:`NewEnumerator6`
        (set `self.Chest_Chance` _returnvalue)
        (set `self.Reward_Combat_Chance` _returnvalue)))))

(event `self.ReceiveTick`
  (params (DeltaSeconds :type "Float (single-precision)"))
  (bind _keys (`BlueprintMapLibrary.Map_Keys` (`self.Player_Stats_Map`)))
  (for _array_element _keys
    (`KismetSystemLibrary.PrintString` (`KismetStringLibrary.Concat_StrStr` (`|GetEnumeratorNameAsString` _array_element) " : " (`KismetStringLibrary.Conv_IntToString` (`BlueprintMapLibrary.Map_Find` (`self.Player_Stats_Map`) _array_element))) true true (struct :`G` 0.66 :`B` 1.0 :`A` 1.0) 0.0)))

(fn `Character_Look_At_Cursor`
  (bind (_returnvalue_roll _returnvalue_pitch _returnvalue_yaw) (`KismetMathLibrary.BreakRotator` (`KismetMathLibrary.FindLookAtRotation` (`self.K2_GetActorLocation` self) (`.Location` (`GameplayStatics.BreakHitResult` (`PlayerController.GetHitResultUnderCursorByChannel` (`GameplayStatics.GetPlayerController` 0) "TraceTypeQuery1" true))))))
  (if (not (`self.Is in HUB?`))
    (`SceneComponent.K2_SetWorldRotation` (`self.CapsuleComponent`) (`KismetMathLibrary.MakeRotator` 0.0 0.0 _returnvalue_yaw) false false)))

(fn `Move Map Menu XAxis`
  (params (Axis_X_Value :type "Float (double-precision)"))
  (bind _outactors (`GameplayStatics.GetAllActorsOfClass` "/Game/RogueLike_Game/Proto/Characters/Player/Widgets/MapMenu/Blueprints/MapMenu_Camera_Actor.MapMenu_Camera_Actor_C"))
  (if (> Axis_X_Value 0.0)
    (bind _output (`|GetArrayItem` _outactors))
    (bind _defaultsceneroot (`/Game/RogueLike_Game/Proto/Characters/Player/Widgets/MapMenu/Blueprints/MapMenu_Camera_Actor.DefaultSceneRoot` _output))
    (bind (_returnvalue_x _returnvalue_y) (`KismetMathLibrary.BreakVector` (`SceneComponent.K2_GetComponentLocation` _defaultsceneroot)))
    (bind _returnvalue (/ (`SceneCaptureComponent2D.OrthoWidth` (`/Game/RogueLike_Game/Proto/Characters/Player/Widgets/MapMenu/Blueprints/MapMenu_Camera_Actor.MapMenu_ComponentCapture` _output)) 200.0))
    (`SceneComponent.K2_SetWorldLocation` _defaultsceneroot (`KismetMathLibrary.MakeVector` (+ _returnvalue_x _returnvalue) (+ _returnvalue_y _returnvalue) -1000.0) false false)
    (elif (< Axis_X_Value 0.0)
      (`SceneComponent.K2_SetWorldLocation` _defaultsceneroot (`KismetMathLibrary.MakeVector` (- _returnvalue_x _returnvalue) (- _returnvalue_y _returnvalue) -1000.0) false false))))

(fn `Move Map Menu YAxis`
  (params (Axis_Y_Value :type "Float (double-precision)"))
  (bind _outactors (`GameplayStatics.GetAllActorsOfClass` "/Game/RogueLike_Game/Proto/Characters/Player/Widgets/MapMenu/Blueprints/MapMenu_Camera_Actor.MapMenu_Camera_Actor_C"))
  (if (> Axis_Y_Value 0.0)
    (bind _output (`|GetArrayItem` _outactors))
    (bind _defaultsceneroot (`/Game/RogueLike_Game/Proto/Characters/Player/Widgets/MapMenu/Blueprints/MapMenu_Camera_Actor.DefaultSceneRoot` _output))
    (bind (_returnvalue_x _returnvalue_y) (`KismetMathLibrary.BreakVector` (`SceneComponent.K2_GetComponentLocation` _defaultsceneroot)))
    (bind _returnvalue (/ (`SceneCaptureComponent2D.OrthoWidth` (`/Game/RogueLike_Game/Proto/Characters/Player/Widgets/MapMenu/Blueprints/MapMenu_Camera_Actor.MapMenu_ComponentCapture` _output)) 200.0))
    (`SceneComponent.K2_SetWorldLocation` _defaultsceneroot (`KismetMathLibrary.MakeVector` (- _returnvalue_x _returnvalue) (+ _returnvalue_y _returnvalue) -1000.0) false false)
    (elif (< Axis_Y_Value 0.0)
      (`SceneComponent.K2_SetWorldLocation` _defaultsceneroot (`KismetMathLibrary.MakeVector` (+ _returnvalue_x _returnvalue) (- _returnvalue_y _returnvalue) -1000.0) false false))))

(fn `UserConstructionScript`)