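; Merc_Armor_BP is an actor, apparently an armor merchant, that sets up three loot items with randomized rarity.
; On BeginPlay it rolls a rarity for each Loot child actor, then writes that rarity plus a fixed loot-system and item type into its Loot_System_Actor_Proto.
; PickRarity uses tiered percentage thresholds offset by StagePercent, always read at key 1 because the Map_Generator_Proto lookup is disconnected.
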(event `self.ReceiveBeginPlay`
  (for _array_element (`|MakeArray` (`self.Loot_01`) (`self.Loot_02`) (`self.Loot_03`))
    (bind _rarity (`self.Pick_Rarity`))
    (set `self.Rarity` _rarity)
    (bind _asloot_system_actor_proto (cast `/Game/RogueLike_Game/Proto/Blueprints/Loot_System/Actor/Loot_System_Actor_Proto` (`ChildActorComponent.ChildActor` _array_element)))
    (set `/Game/RogueLike_Game/Proto/Blueprints/Loot_System/Actor/Loot_System_Actor_Proto.Loot_System_Type` "NewEnumerator3" _asloot_system_actor_proto)
    (set `/Game/RogueLike_Game/Proto/Blueprints/Loot_System/Actor/Loot_System_Actor_Proto.Item_Type` "NewEnumerator8" _asloot_system_actor_proto)
    (set `/Game/RogueLike_Game/Proto/Blueprints/Loot_System/Actor/Loot_System_Actor_Proto.Item_Rarity` (`self.Rarity`) _asloot_system_actor_proto)))

(fn `Pick_Rarity`
  (returns (Rarity :type "/Game/RogueLike_Game/Proto/Blueprints/Loot_System/Actor/Utilities/Enum/Rarity_Enum Enum"))
  (locals (Stage_Percent :type "Map of Integer to Integer") (Percent :type Integer))
  (bind _value (`BlueprintMapLibrary.Map_Find` (`local.Stage_Percent`) 1))
  (bind _output_get (set `local.Percent` (`KismetMathLibrary.RandomIntegerInRange` 1 100)))
  (if (<= _output_get (+ 0 _value))
    (return "NewEnumerator3")
    (elif (<= (`local.Percent`) (+ 20 _value))
      (return "NewEnumerator2")
      (elif (<= (`local.Percent`) (+ 50 _value))
        (return "NewEnumerator1")
        (else
          (return "NewEnumerator0"))))))

(fn `UserConstructionScript`)